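; BatTestPlayerController is a test player controller that drives its player automatically with simulated input.
; A looping timer started on BeginPlay fires JumpAndFire every second, briefly holding left mouse, space bar and a direction key before releasing them.
; After each release the stored direction key alternates between Left and Right, so presumably the player jumps and fires while moving side to side.
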(event Custom|JumpAndFire
  (bind _self self)
  (bind _self_2 self)
  ;[1 1 1] Comment
  (Class|ShooterPlayerController|SimulateInputKey _self "LeftMouseButton" true)
  (Class|ShooterPlayerController|SimulateInputKey _self "SpaceBar" true)
  (Class|ShooterPlayerController|SimulateInputKey _self (Variables|Default|GetDirect) true)
  (Utilities|FlowControl|Delay 0.2)
  (Class|ShooterPlayerController|SimulateInputKey _self_2 "LeftMouseButton" false)
  (Class|ShooterPlayerController|SimulateInputKey _self_2 "SpaceBar" false)
  (Class|ShooterPlayerController|SimulateInputKey _self_2 (Variables|Default|GetDirect) false)
  (if (== (Variables|Default|GetDirect) "Left")
    (Variables|Default|SetDirect "Right")
    (else
      (Variables|Default|SetDirect "Left"))))

(event EventBeginPlay
  ;[1 1 1] Comment
  (Utilities|Time|SetTimerbyEvent (delegate Custom|JumpAndFire) 1.0 true))

(event EventTick
  (params (DeltaSeconds :type Float%20%28single-precision%29)))

(fn ConstructionScript)